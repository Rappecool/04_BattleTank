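; Tank_BP is the player-controllable tank pawn, wiring input to aiming and movement components.
; On BeginPlay it hands the barrel and turret to TankAiming and both tracks to TankMovement, with debug prints.
; Aim axes rotate an azimuth gimbal and spring arm at a frame-rate-independent speed to orbit the camera.
; Move and turn axes pass intent to TankMovement, and Fire triggers TankAiming.
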(event `self.ReceiveBeginPlay`
  (`KismetSystemLibrary.PrintString` "Tank_BP BeginPLay Called")
  (`TankAimingComponent.Initialise` (`self.TankAiming`) (`self.TankBarrel`) (`self.TankTurret`))
  (`KismetSystemLibrary.PrintString` "Initalise Aiming in BP called.")
  (`TankMovementComponent.Initialise` (`self.TankMovement`) (`self.LeftTrack`) (`self.RightTrack`))
  (`KismetSystemLibrary.PrintString` "Initalise Movement in BP called."))

(event `InputAxis|AimAzimuth`
  (params (AxisValue :type "Float (single-precision)"))
  ;[1 1 1] Aim Binding
  (`SceneComponent.K2_AddLocalRotation` (`self.Azimuth Gimbal`) (`KismetMathLibrary.MakeRotator` 0.0 0.0 (* AxisValue (`GameplayStatics.GetWorldDeltaSeconds`) 100.0)) false false))

(event `InputAxis|AimElevation`
  (params (AxisValue :type "Float (single-precision)"))
  ;[1 1 1] Aim Binding
  (`SceneComponent.K2_AddLocalRotation` (`self.SpringArm`) (`KismetMathLibrary.MakeRotator` 0.0 (* AxisValue (`GameplayStatics.GetWorldDeltaSeconds`) 100.0)) false false))

(event `InputAxis|MoveForward`
  (params (AxisValue :type "Float (single-precision)"))
  ;[1 1 1] Movement Input Binding
  (`TankMovementComponent.IntendMoveForward` (`self.TankMovement`) AxisValue))

(event `InputAxis|Turn Right`
  (params (AxisValue :type "Float (single-precision)"))
  ;[1 1 1] Movement Input Binding
  (`TankMovementComponent.IntendTurnRight` (`self.TankMovement`) AxisValue))

(event `InputAction|Fire`
  (params (Key :type "Key Structure" :default "AnyKey"))
  ;[1 1 1] Aim Binding
  (:`Pressed`
    (`TankAimingComponent.Fire` (`self.TankAiming`))))

(fn `UserConstructionScript`
  (`KismetSystemLibrary.PrintString` "Tank_BP Constructor called"))